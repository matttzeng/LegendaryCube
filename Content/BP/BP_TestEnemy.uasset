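; BP_TestEnemy is a test enemy that shoots at the player and can be killed by bullets.
; Tick runs through a half-second Delay, then spawns a BP_bullet at its mesh, aimed at the player's BP_TopDownCharacter capsule.
; Mesh hits print HP and check it against the bullet's Damage, destroying both actors on a lethal hit.
; HP is never decremented, so damage does not accumulate.
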(event `self.ReceiveTick`
  (params (DeltaSeconds :type "Float (single-precision)"))
  (bind _returnvalue (`SceneComponent.K2_GetComponentLocation` (`self.StaticMesh`)))
  (`KismetSystemLibrary.Delay` 0.5)
  (bind _asbp_top_down_character (cast `/Game/TopDown/Blueprints/BP_TopDownCharacter` (`GameplayStatics.GetPlayerCharacter` 0)))
  (`|SpawnActorFromClass` "/Game/BP/BP_bullet.BP_bullet_C" (`KismetMathLibrary.MakeTransform` _returnvalue (`KismetMathLibrary.Conv_VectorToRotator` (- (`SceneComponent.K2_GetComponentLocation` (`Character.CapsuleComponent` _asbp_top_down_character)) _returnvalue))) "Undefined" "OverrideRootScale" null null))

(event `self.StaticMesh.OnComponentHit`
  (params (HitComponent :type "PrimitiveComponent Object Reference") (OtherActor :type "Actor Object Reference") (OtherComp :type "PrimitiveComponent Object Reference") (NormalImpulse :type "Vector Structure") (Hit :type "HitResult Structure (by ref)"))
  (`KismetSystemLibrary.PrintString` (`KismetStringLibrary.Conv_IntToString` (`self.HP`)))
  (bind _asbp_bullet (cast `/Game/BP/BP_bullet` OtherActor))
  (if (<= (- (`self.HP`) (`/Game/BP/BP_bullet.Damage` _asbp_bullet)) 0)
    (`self.K2_DestroyActor` OtherActor)
    (`self.K2_DestroyActor`)))

(fn `UserConstructionScript`)